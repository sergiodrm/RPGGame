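; GA_Attack is a Gameplay Ability for a light melee attack with an optional second combo hit.
; It commits and plays the first slash montage section, and an input press during it queues the second slash, which commits again at blend out.
; While active, it listens to the RPGCharacter melee hit delegate to apply the light attack effect to hit actors, unbinding when the ability ends.
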(event `self.K2_OnEndAbility`
  (params (bWasCancelled :type Boolean))
  (remove `RPGCharacter.OnHitMeleeAttackDelegate` (stale `self.K2_ActivateAbility` _asrpgcharacter) (delegate `OnAttackHit`)))

(event `self.K2_ActivateAbility`
  (set `self.UseMeleeCombo` false)
  (bind _returnvalue (`self.K2_CommitAbility`))
  (if _returnvalue
    (`|ExecutionSequence`
      (:`then_0`
        (bind _asrpgcharacter (cast `RPGCharacter` (`.AvatarActor` (break `GameplayAbilityActorInfo` (`self.GetActorInfo`)))))
        (add `RPGCharacter.OnHitMeleeAttackDelegate` _asrpgcharacter (delegate `OnAttackHit`)))
      (:`then_1`
        (`AbilityTask_PlayMontageAndWait.CreatePlayMontageAndWaitProxy` "None" "/Game/Blueprints/Animation/Player/AM_LightAttackCombo.AM_LightAttackCombo" 1.0 "Slash01"
          (:`then`
            (`AbilityTask_WaitInputPress.WaitInputPress` false
              (:`OnPress`
                (set `self.UseMeleeCombo` true))))
          (:`OnBlendOut`
            (if (`self.UseMeleeCombo`)
              (bind _returnvalue_2 (`self.K2_CommitAbility`))
              (if _returnvalue_2
                (`AbilityTask_PlayMontageAndWait.CreatePlayMontageAndWaitProxy` "None" "/Game/Blueprints/Animation/Player/AM_LightAttackCombo.AM_LightAttackCombo" 1.0 "Slash02"
                  (:`OnCompleted`
                    _)
                  (:`OnInterrupted`
                    _)
                  (:`OnCancelled`
                    _))))
            (`self.K2_EndAbility` :!label _label))
          (:`OnInterrupted`
            (goto _label))
          (:`OnCancelled`
            (goto _label)))))
    (else
      (goto _label))))

(event `OnAttackHit`
  (params (hitActor :type "Actor Object Reference"))
  (`self.BP_ApplyGameplayEffectToTarget` (`AbilitySystemBlueprintLibrary.AbilityTargetDataFromActor` hitActor) "/Game/Blueprints/AbilitySystem/Effects/GE_LightAttackTarget.GE_LightAttackTarget_C"))